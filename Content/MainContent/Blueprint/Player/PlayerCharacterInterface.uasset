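; Blueprint interface for the player character, exposing player and weapon state to other assets without a direct cast.
; Getters cover firing, zooming, sprinting, moving and reloading states, plus reload rate, zoom timing and progress, ammo counts, volume setting and a bolt follower origin.
; CallOnHit, which passes a hit location, and CallOnKill let callers notify the player of hits and kills.
; All functions are empty declarations for implementers to fill.
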(fn GetIsPlayerFiring
  (return false))

(fn GetVolumeSetting
  (return 0.0))

(fn GetIsPlayerZooming
  (return false))

(fn GetIsPlayerSprinting
  (return false))

(fn GetIsPlayerMoving
  (return false))

(fn GetIsPlayerReloading
  (return false))

(fn GetReloadRate
  (return 0.0))

(fn GetZoomTiming
  (return 0.0 0.0))

(fn GetAmmoCounts
  (return 0 0))

(fn CallonHit
  (params (HitLocation :type Vector)))

(fn CallonKill)

(fn GetPlayerZoomProgress
  (return 0.0))

(fn GetBoltFollowerOrigin
  (return "0, 0, 0"))