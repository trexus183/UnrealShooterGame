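; EnemyController is the AI controller for enemy characters, running their behavior tree on possession and registering itself as the pawn's parent controller.
; Perception updates set line-of-sight and target Blackboard keys when an actor tagged Player is sensed.
; Any other perception update starts a delayed timer that clears both keys, and re-sensing the player cancels it, giving enemies a grace period before losing their target.
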(event OnTargetPerceptionUpdated(Perception)
  (params (Actor :type Actor%20Object%20Reference) (Stimulus :type AI%20Stimulus%20Structure))
  (bind _blackboard (Variables|Default|GetBlackboard))
  ;[1 1 1] Perception Update
  (if (and (Actor|ActorHasTag Actor "Player") (.bSuccessfullySensed (Utilities|Struct|BreakAIStimulus Stimulus)))
    (Utilities|Time|ClearandInvalidateTimerbyHandle (Variables|Default|GetLosResetTimer))
    (AI|Components|Blackboard|SetValueasBool _blackboard (Variables|Default|GetHasLineOfSight) true)
    (AI|Components|Blackboard|SetValueasObject _blackboard (Variables|Default|GetEnemyActor) Actor)
    (else
      (bind _returnvalue (Utilities|Time|SetTimerbyEvent (delegate Custom|ResetLos) (Variables|Default|GetLOSTimerDelay)))
      (Variables|Default|SetLosResetTimer _returnvalue))))

(event Custom|ResetLos
  (bind _blackboard (Variables|Default|GetBlackboard))
  ;[1 1 1] Perception Update
  (AI|Components|Blackboard|SetValueasBool _blackboard (Variables|Default|GetHasLineOfSight) false)
  (AI|Components|Blackboard|SetValueasObject _blackboard (Variables|Default|GetEnemyActor) 0))

(event EventPossess
  (params (PossessedPawn :type Pawn%20Object%20Reference))
  ;[1 1 1] On Posses
  (AI|RunBehaviorTree "/Game/MainContent/Blueprint/Enemies/EnemyBehaviorTree.EnemyBehaviorTree")
  (bind _asenemy_character (Utilities|Casting|CastToEnemyCharacter PossessedPawn))
  (Variables|/Game/MainContent/Blueprint/Enemies/EnemyCharacter.EnemyCharacter_C|SetParentController _asenemy_character self))

(fn ConstructionScript)