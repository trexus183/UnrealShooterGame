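; Base enemy character that takes projectile hits, shows a name and health label, and dies with ragdoll.
; RecieveHit treats hits near the headshot sphere as criticals, plays a hit sound, alerts the AI controller to the player, and spawns floating damage text.
; Health changes set flags that Tick consumes to play normal or critical death, mark the blackboard dead, ragdoll, then destroy.
; Overlap with the player car deals speed-based damage of at least max health.
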(event OnComponentBeginOverlap(CapsuleComponent)
  (params (OverlappedComponent :type Primitive%20Component%20Object%20Reference) (OtherActor :type Actor%20Object%20Reference) (OtherComp :type Primitive%20Component%20Object%20Reference) (OtherBodyIndex :type Integer) (bFromSweep :type Boolean) (SweepResult :type Hit%20Result%20Structure%20%28by%20ref%29))
  (bind _asplayer_car (Utilities|Casting|CastToplayerCar OtherActor))
  (CallFunction|RecieveDamage (Math|Float|Clamp(Float) (Math|Vector|VectorLength (Transformation|GetVelocity _asplayer_car)) (Variables|Default|GetMaxHealth) 999999.0) false (Transformation|GetWorldLocation (Variables|Default|GettorsoCollider)))
  (Physics|SetSimulatePhysics (Variables|Character|GetMesh) true))

(event EventTick
  (params (DeltaSeconds :type Float%20%28single-precision%29))
  (Variables|Default|SetCanPlayHitSound true)
  (if (Variables|Default|GetPlayHitReact)
    (Variables|Default|SetPlayHitReact false)
    (elif (Variables|Default|GetPlayDeathReaction)
      (Variables|Default|SetPlayDeathReaction false)
      (Components|Animation|PlayAnimation (Variables|Character|GetMesh) "/Game/MainContent/Animation/ThirdPerson/Death_1.Death_1" false)
      (bind _asenemy_controller (Utilities|Casting|CastToEnemyController (Variables|Default|GetParentController) :!label _label))
      (AI|Components|Blackboard|SetValueasBool (AI|GetBlackboard _asenemy_controller) (Variables|Default|GetIsDeadBlackboardValue) true)
      (Rendering|SetVisibility (Variables|Default|GetName%20Text) false false)
      (Collision|SetCollisionEnabled (Variables|Default|GetHeadshotCollider) "PhysicsOnly")
      (Collision|SetCollisionEnabled (Variables|Collision|GetCapsuleComponent) "NoCollision")
      (Utilities|FlowControl|Delay 0.8)
      (Physics|SetSimulatePhysics (Variables|Character|GetMesh) true)
      (Utilities|FlowControl|Delay 8.0)
      (Actor|DestroyActor)
      (elif (Variables|Default|GetPlayCritDeathReaction)
        (Variables|Default|SetPlayCritDeathReaction false)
        (Components|Animation|PlayAnimation (Variables|Character|GetMesh) "/Game/MainContent/Animation/ThirdPerson/Death_3.Death_3" false)
        (bind _returnvalue (AddComponent|AddNiagaraComponent false))
        (Transformation|SetWorldLocation _returnvalue (Transformation|GetWorldLocation (Variables|Default|GetHeadshotCollider)) false false)
        (goto _label)))))

(event EventBeginPlay
  (CallFunction|SetHealth (Variables|Default|GetMaxHealth) false))

(fn ConstructionScript)

(fn UpdateWalkSpeed
  (params (NewWalkSpeed :type Float%20%28single-precision%29))
  (Variables|/Script/Engine.CharacterMovementComponent|SetMaxWalkSpeed (Variables|Character|GetCharacterMovement) NewWalkSpeed))

(fn RecieveHit
  (params (HitLocation :type Vector) (Damage :type Float%20%28single-precision%29) (BoltSize :type Float%20%28single-precision%29) (CritMultiplier :type Float%20%28single-precision%29))
  (if (>= (Variables|Default|GetHealth) 0.0)
    (bind _returnvalue (AddComponent|AddNiagaraComponent false))
    (Transformation|SetWorldLocation _returnvalue HitLocation false true)
    (if (<= (Math|Vector|Distance(Vector) HitLocation (Transformation|GetWorldLocation (Variables|Default|GetHeadshotCollider))) (+ BoltSize (Variables|/Script/Engine.SphereComponent|GetSphereRadius (Variables|Default|GetHeadshotCollider))))
      (CallFunction|RecieveDamage (* Damage CritMultiplier) true HitLocation)
      (if (Variables|Default|GetCanPlayHitSound)
        (bind _volume (Class|PlayerCharacterInterface|GetVolumeSetting(Message) (Game|Player|GetPlayerPawn 0)))
        (Audio|PlaySound2D "/Game/MainContent/Audio/hitSound.hitSound" (* _volume 2.0) 1.5 0.0 0 0)
        (Variables|Default|SetCanPlayHitSound false)
        (bind _asenemy_controller (Utilities|Casting|CastToEnemyController (Variables|Default|GetParentController) :!label _label))
        (Utilities|Time|ClearandInvalidateTimerbyHandle (Variables|/Game/MainContent/Blueprint/Enemies/EnemyController.EnemyController_C|GetLosResetTimer _asenemy_controller))
        (AI|Components|Blackboard|SetValueasBool (Variables|/Script/AIModule.AIController|GetBlackboard _asenemy_controller) (Variables|/Game/MainContent/Blueprint/Enemies/EnemyController.EnemyController_C|GetHasLineOfSight _asenemy_controller) true)
        (AI|Components|Blackboard|SetValueasObject (Variables|/Script/AIModule.AIController|GetBlackboard _asenemy_controller) (Variables|/Game/MainContent/Blueprint/Enemies/EnemyController.EnemyController_C|GetEnemyActor _asenemy_controller) (Game|Player|GetPlayerPawn 0)))
      (else
        (CallFunction|RecieveDamage Damage false HitLocation)
        (if (Variables|Default|GetCanPlayHitSound)
          (bind _volume_2 (Class|PlayerCharacterInterface|GetVolumeSetting(Message) (Game|Player|GetPlayerPawn 0)))
          (Audio|PlaySound2D "/Game/MainContent/Audio/hitSound.hitSound" (* _volume_2 2.0) 1.0 0.0 0 0)
          (Variables|Default|SetCanPlayHitSound false)
          (goto _label))))))

(fn SetHealth
  (params (Health :type Float%20%28single-precision%29) (WasCiriticalDamage :type Boolean))
  (Variables|Default|SetHealth Health)
  (Rendering|Components|TextRender|SetText (Variables|Default|GetName%20Text) (Utilities|Text|ToText(String) (Utilities|String|Append (Variables|Default|GetName) ": " (Utilities|String|ToString(Integer) (Class|KismetMathLibrary|FCeil64 (Variables|Default|GetHealth))) "/" (Utilities|String|ToString(Integer) (Class|KismetMathLibrary|FCeil64 (Variables|Default|GetMaxHealth))))))
  (if (<= (Variables|Default|GetHealth) 0.0)
    (if WasCiriticalDamage
      (Variables|Default|SetPlayCritDeathReaction true)
      (else
        (Variables|Default|SetPlayDeathReaction true)))
    (Class|PlayerCharacterInterface|CallonKill(Message) (Game|Player|GetPlayerPawn 0))
    (else
      (Variables|Default|SetPlayHitReact true))))

(fn RecieveDamage
  (params (Damage :type Float%20%28single-precision%29) (HitWasCritical :type Boolean) (HitLocation :type Vector))
  (CallFunction|SetHealth (- (Variables|Default|GetHealth) Damage) HitWasCritical)
  (bind _returnvalue (Game|SpawnActorfromClass "/Game/MainContent/Blueprint/DamageText.DamageText_C" (Math|Transform|MakeTransform HitLocation (Transformation|GetWorldRotation (Variables|Collision|GetCapsuleComponent)) "1,1,1") "Undefined" 0 0))
  (Default|SetText _returnvalue Damage HitWasCritical))