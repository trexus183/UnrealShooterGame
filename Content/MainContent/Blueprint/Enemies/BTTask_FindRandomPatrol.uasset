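; Behavior tree task that picks a random patrol destination for an EnemyCharacter.
; It sets the pawn's walk speed to PatrolSpeed, then writes a reachable point within a fixed radius of the pawn to PatrolLocationKey.
; If no point is found, it stores the pawn's current location and still succeeds.
; The task fails only when the pawn is not an EnemyCharacter.
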(event EventReceiveExecuteAI
  (params (OwnerController :type AI%20Controller%20Object%20Reference) (ControlledPawn :type Pawn%20Object%20Reference))
  (bind _returnvalue (Transformation|GetActorLocation ControlledPawn))
  (bind (_randomlocation _returnvalue_2) (AI|Navigation|GetRandomReachablePointinRadius _returnvalue 5e+02 0 0))
  (bind _asenemy_character (Utilities|Casting|CastToEnemyCharacter ControlledPawn)
    (:then
      (Default|UpdateWalkSpeed _asenemy_character (Variables|Default|GetPatrolSpeed))
      (if _returnvalue_2
        (AI|BehaviorTree|SetBlackboardValueasVector (Variables|Default|GetPatrolLocationKey) _randomlocation)
        (else
          (AI|BehaviorTree|SetBlackboardValueasVector (Variables|Default|GetPatrolLocationKey) _returnvalue)))
      (AI|BehaviorTree|FinishExecute true))
    (:CastFailed
      (AI|BehaviorTree|FinishExecute false))))