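; Behavior tree task named for an enemy attacking the player, currently inert because its execute event is wired to nothing.
; Disconnected logic would spawn a Bolt at the EnemyCharacter's BoltOrigin, mark the shooter as allied, set damage and zero gravity, and launch it forward by impulse.
; Both FinishExecute calls are also unreachable, so the task never reports completion.
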(event EventReceiveExecuteAI
  (params (OwnerController :type AI%20Controller%20Object%20Reference) (ControlledPawn :type Pawn%20Object%20Reference)))