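; Bolt follower actor that draws a cable trail from the farthest bolt location back toward a player-supplied origin, capped at a maximum length.
; Tick refreshes the origin while nearby, moves the actor to the bolt location and fades the cable in beyond a hide distance.
; When the bolt becomes invalid, it ensures the trail becomes visible, then fades and shrinks it via timeline before destroying itself.
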(event EventBeginPlay
  ;[1 1 1] Begin Play
  (Variables|Default|SetOriginPoint (Transformation|GetWorldLocation (Variables|Default|GetCable)))
  (Utilities|FlowControl|Delay 0.0)
  (Variables|/Script/CableComponent.CableComponent|SetCableWidth (Variables|Default|GetCable) (Variables|Default|GetCableWidth)))

(event EventTick
  (params (DeltaSeconds :type Float%20%28single-precision%29))
  ;[1 1 1] Tick
  (if (Variables|Default|GetFollowerShouldDestroy)
    ;[1 1 1] Hide If Showing Gate
    (if (>= (Variables|Default|GetPeakOpacity) (* (Variables|Default|GetOpacityCap) 0.1))
      ;[1 1 1] Hide On Bolt Death
      (Audio|Components|Audio|Stop (Variables|Default|GetFadeInTimeline))
      (bind (_direction _opacity _cablelength) (Timeline|FadeOutTimeline Play)
        (:Update
          (Rendering|Material|SetScalarParameterValueonMaterials (Variables|Default|GetCable) "Opacity" (* _opacity (Variables|Default|GetPeakOpacity)))
          (Variables|/Script/CableComponent.CableComponent|SetEndLocation (Variables|Default|GetCable) (* (Math|Vector|Normalize (- (Variables|Default|GetOriginPoint) (Variables|Default|GetFarthestBoltLocation))) (* _cablelength (Variables|Default|GetPeakCableLength)))))
        (:Finished
          (Utilities|FlowControl|Delay 0.5)
          (Actor|DestroyActor)))
      (elif (not (Variables|Default|GetIsShowing))
        ;[1 1 1] Show If Hidden
        (Variables|Default|SetIsShowing true :!label _label)
        (Utilities|FlowControl|Sequence
          (:then_0
            ;[1 1 1] Update Cable Length
            (Transformation|SetActorLocation (Variables|Default|GetFarthestBoltLocation) false false :!label _label_2)
            (Variables|/Script/CableComponent.CableComponent|SetEndLocation (Variables|Default|GetCable) (* (Math|Vector|Normalize (- (Variables|Default|GetOriginPoint) (Variables|Default|GetFarthestBoltLocation))) (Math|Float|Clamp(Float) (Math|Vector|VectorLength (- (Variables|Default|GetOriginPoint) (Variables|Default|GetFarthestBoltLocation))) 0.0 (Variables|Default|GetMaxLength))))
            (Variables|Default|SetPeakCableLength (Math|Float|Clamp(Float) (Math|Vector|VectorLength (- (Variables|Default|GetOriginPoint) (Variables|Default|GetFarthestBoltLocation))) 0.0 (Variables|Default|GetMaxLength))))
          (:then_1
            (bind _opacity_2 (Timeline|FadeinTimeline PlayFromStart)
              (:Update
                (Rendering|Material|SetScalarParameterValueonMaterials (Variables|Default|GetCable) "Opacity" (* _opacity_2 (Variables|Default|GetOpacityCap)))
                (Variables|Default|SetPeakOpacity (* _opacity_2 (Variables|Default|GetOpacityCap)))))))))
    (else
      (if (<= (Math|Vector|VectorLength (- (Variables|Default|GetOriginPoint) (Variables|Default|GetFarthestBoltLocation))) (* (Variables|Default|GetMaxLength) 2.0))
        (bind _boltfollowerorigin (Class|PlayerCharacterInterface|GetBoltFollowerOrigin(Message) (Game|GetPlayerCharacter 0)))
        (Variables|Default|SetOriginPoint _boltfollowerorigin))
      (Utilities|IsValid (Variables|Default|GetBolt)
        (:Is%20Valid
          _)
        (:Is%20Not%20Valid
          (Variables|Default|SetFollowerShouldDestroy true)))
      (if (Variables|Default|GetIsShowing)
        (goto _label_2)
        (elif (>= (Math|Vector|VectorLength (- (Variables|Default|GetOriginPoint) (Variables|Default|GetFarthestBoltLocation))) (Variables|Default|GetHideDistance))
          (goto _label))))))

(fn ConstructionScript)