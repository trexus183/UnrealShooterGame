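; DamageText is a floating damage number shown in the world, with SetText writing the floored damage and applying a separate color for critical hits.
; BeginPlay picks random sideways (world Y) and upward velocities, with ranges that widen with distance from the player pawn.
; Tick moves the text until drift stops after half a second, while continually scaling it by distance and rotating it to face the player.
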(event EventBeginPlay
  (bind _returnvalue (Game|Player|GetPlayerPawn 0))
  (bind _damagetext (Variables|Default|GetDamageText))
  (bind _returnvalue_2 (Transformation|GetWorldLocation _damagetext))
  (bind _returnvalue_3 (Transformation|GetActorLocation _returnvalue))
  (bind _returnvalue_4 (Math|Vector|Distance(Vector) _returnvalue_2 _returnvalue_3))
  (bind _returnvalue_5 (/ _returnvalue_4 2e+01))
  (bind _returnvalue_6 (+ _returnvalue_5 75.0))
  ;[1 1 1] Begin Play
  (Variables|Default|SetVelocityY (Math|Random|RandomFloatinRange (* _returnvalue_6 -1.0) _returnvalue_6))
  (Variables|Default|SetVelocityZ (Math|Random|RandomFloatinRange 5e+01 _returnvalue_6)))

(event EventTick
  (params (DeltaSeconds :type Float%20%28single-precision%29))
  (bind _returnvalue (Game|Player|GetPlayerPawn 0))
  (bind _damagetext (Variables|Default|GetDamageText))
  (bind _returnvalue_2 (Transformation|GetActorLocation _returnvalue))
  ;[1 1 1] Event Tick
  (Transformation|SetWorldLocation _damagetext (+ (Transformation|GetWorldLocation _damagetext) (Math|Vector|MakeVector 0.0 (* (Variables|Default|GetVelocityY) DeltaSeconds) (* (Variables|Default|GetVelocityZ) DeltaSeconds))) false false)
  (Rendering|Components|TextRender|SetWorldSize (Variables|Default|GetDamageText) (/ (Math|Vector|Distance(Vector) (Transformation|GetWorldLocation (Variables|Default|GetDamageText)) _returnvalue_2) 25.0))
  (Transformation|SetWorldRotation (Variables|Default|GetDamageText) (Math|Rotator|MakeRotfromX (Math|Vector|Normalize (- _returnvalue_2 (Transformation|GetWorldLocation (Variables|Default|GetDamageText))))) false false)
  (bind _output_get (Variables|Default|SetExistenceTime (+ (Variables|Default|GetExistenceTime) DeltaSeconds)))
  (if (>= _output_get 0.5)
    (Variables|Default|SetVelocityY 0.0)
    (Variables|Default|SetVelocityZ 0.0)))

(fn ConstructionScript)

(fn SetText
  (params (Damage :type Float%20%28single-precision%29) (IsCritical :type Boolean))
  (Rendering|Components|TextRender|SetText (Variables|Default|GetDamageText) (Utilities|Text|ToText(Integer) (Math|Float|Floor Damage)))
  (if IsCritical
    (Rendering|Components|TextRender|SetTextRenderColor (Variables|Default|GetDamageText) (Variables|Default|GetCritDamageColor))))