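; Bolt is a physics-driven projectile that damages enemies and destroys itself on hitting a valid non-allied actor.
; Each tick it applies a frame-rate-scaled downward impulse as custom gravity, then sphere-traces from its previous location to avoid tunneling.
; Pawn traces use the collider's radius while object traces use a thin one, both ignoring allied pawns.
; Hits pass damage, bolt size and crit multiplier to tagged enemies and notify the player pawn.
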(event EventTick
  (params (DeltaSeconds :type Float%20%28single-precision%29))
  (bind _spherecollider (Variables|Default|GetSphereCollider))
  ;[1 1 1] Event Tick
  (bind _output_get (Variables|Default|SetDeltaTime DeltaSeconds))
  (Variables|Default|SetDeltaTimeProportion (/ _output_get 0.016))
  (CallFunction|SimulateGravity)
  (CallFunction|ContinuousCollisionCheck)
  (Utilities|IsValid _spherecollider
    (:Is%20Valid
      (Variables|Default|SetPreviousLocation (Transformation|GetWorldLocation _spherecollider))
      (if (Variables|Default|GetHasCollided)
        _))))

(event EventBeginPlay
  ;[1 1 1] Begin Play
  (Rendering|SetVisibility (Variables|Default|GetBoltMesh) false false)
  (Utilities|FlowControl|Delay 0.016)
  (Rendering|SetVisibility (Variables|Default|GetBoltMesh) true false))

(fn ConstructionScript)

(fn SimulateGravity
  (bind _spherecollider (Variables|Default|GetSphereCollider))
  (Physics|AddImpulse _spherecollider (* (Math|Vector|GetUpVector _spherecollider) (* (Variables|Default|GetGravityScale) -0.098 (Variables|Default|GetDeltaTimeProportion))) "None" false))

(fn HandleCollision
  (params (HitActor :type Actor%20Object%20Reference) (HitLocation :type Vector))
  (Utilities|IsValid HitActor
    (:Is%20Valid
      (if (not (Utilities|Array|ContainsItem (Variables|Default|GetAlliedPawns) HitActor))
        (if (Actor|ActorHasTag HitActor "Enemy")
          (bind _asenemy_character (Utilities|Casting|CastToEnemyCharacter HitActor))
          (Default|RecieveHit _asenemy_character HitLocation (Variables|Default|GetDamage) (Variables|/Script/Engine.SphereComponent|GetSphereRadius (Variables|Default|GetSphereCollider)) (Variables|Default|GetCritMultiplier)))
        (Class|PlayerCharacterInterface|CallonHit(Message) (Game|Player|GetPlayerPawn 0) HitLocation)
        (Actor|DestroyActor)))))

(fn ContinuousCollisionCheck
  (if (Utilities|Operators|NotEqual(!=) :A (Variables|Default|GetPreviousLocation) :ErrorTolerance 0.001)
    ;[1 1 1] Trace For Pawns
    (bind (_outhit _returnvalue) (Collision|SphereTraceForObjects (Variables|Default|GetPreviousLocation) (Transformation|GetWorldLocation (Variables|Default|GetSphereCollider)) (Variables|/Script/Engine.SphereComponent|GetSphereRadius (Variables|Default|GetSphereCollider)) (Variables|Default|GetCollisionTracePawnTypes) false (Variables|Default|GetAlliedPawns) "None" true "(R=1.000000,G=0.000000,B=0.000000,A=1.000000)" "(R=0.000000,G=1.000000,B=0.000000,A=1.000000)" 3.0))
    (if _returnvalue
      (CallFunction|HandleCollision (.HitActor (Collision|BreakHitResult _outhit)) (.ImpactPoint (Collision|BreakHitResult _outhit)))
      ;[1 1 1] Trace For Objects
      (Utilities|IsValid (Variables|Default|GetSphereCollider)
        (:Is%20Valid
          _)))
    (bind (_outhit_2 _returnvalue_2) (Collision|SphereTraceForObjects (Variables|Default|GetPreviousLocation) (Transformation|GetWorldLocation (Variables|Default|GetSphereCollider)) 0.5 (Variables|Default|GetCollisionTraceObjectTypes) false (Variables|Default|GetAlliedPawns) "None" true "(R=1.000000,G=0.000000,B=0.000000,A=1.000000)" "(R=0.000000,G=1.000000,B=0.000000,A=1.000000)" 3.0))
    (if _returnvalue_2
      (CallFunction|HandleCollision (.HitActor (Collision|BreakHitResult _outhit_2)) (.Location (Collision|BreakHitResult _outhit_2))))))