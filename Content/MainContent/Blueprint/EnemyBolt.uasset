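; EnemyBolt is an enemy bolt Blueprint that builds on inherited BeginPlay logic.
; After a zero-length delay, it scales BoltMesh uniformly from the SphereCollider radius so the visual follows the collision size, then sets IsEnemyBolt to true.
; It adds no overlap or tick logic of its own, and its construction script only calls the parent.
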(event EventBeginPlay
  (bind _spherecollider (Variables|Default|GetSphereCollider))
  (bind _sphereradius (Variables|/Script/Engine.SphereComponent|GetSphereRadius _spherecollider))
  (bind _returnvalue (/ _sphereradius 5e+01))
  (|CallParentFunction)
  (Utilities|FlowControl|Delay 0.0)
  (Transformation|SetRelativeScale3D (Variables|Default|GetBoltMesh) (Math|Vector|MakeVector _returnvalue _returnvalue _returnvalue))
  (Variables|Default|SetIsEnemyBolt true))

(event Collision|EventActorBeginOverlap
  (params (OtherActor :type Actor%20Object%20Reference)))

(event EventTick
  (params (DeltaSeconds :type Float%20%28single-precision%29))
  (|CallParentFunction DeltaSeconds) ; This node is disabled and will not be called.\nDrag off pins to build functionality.
)

(fn ConstructionScript
  (|CallParentFunction))